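; BP_DamageBlock is an actor that, despite its name, restores mana to the player who hits it.
; When its Sphere1 component registers a hit from BP_TestPlayer and that player's mana is below maximum, it adds a fixed amount clamped to MaxMana.
; It then destroys itself and prints a debug message, staying in place if mana is already full.
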(event `self.Sphere1.OnComponentHit`
  (params (HitComponent :type "PrimitiveComponent Object Reference") (OtherActor :type "Actor Object Reference") (OtherComp :type "PrimitiveComponent Object Reference") (NormalImpulse :type "Vector Structure") (Hit :type "HitResult Structure (by ref)"))
  (bind _asbp_test_player (cast `/Game/Player/BP_TestPlayer` OtherActor))
  (if (< (`/Game/Player/BP_TestPlayer.Mana` _asbp_test_player) (`/Game/Player/BP_TestPlayer.MaxMana` _asbp_test_player))
    (set `/Game/Player/BP_TestPlayer.Mana` (`KismetMathLibrary.FClamp` (+ (`/Game/Player/BP_TestPlayer.Mana` _asbp_test_player) 5.0) 0.0 (`/Game/Player/BP_TestPlayer.MaxMana` _asbp_test_player)) _asbp_test_player)
    (`self.K2_DestroyActor`)
    (`KismetSystemLibrary.PrintString` "Dodano manę")))

(fn `UserConstructionScript`)