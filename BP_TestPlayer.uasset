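; Test player character that switches between a direct-control camera and a top-down click-to-move camera, each with its own zoom.
; Enhanced Input drives movement, jump, crouch, sprint and aim, while Tick steers toward clicked points until close.
; Aiming enables wand shots of two switchable projectile types with separate cooldowns, and a screen-center trace holds BP_Interactable actors while Interact is pressed.
; BeginPlay adds the input mapping and minimap widget.
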(event `EnhancedInput|/Game/Input/IA_Zoom`
  (params (ActionValue :type "Float (double-precision)") (ElapsedSeconds :type "Float (double-precision)") (TriggeredSeconds :type "Float (double-precision)") (InputAction :type "InputAction Object Reference" :default "/Game/Input/IA_Zoom.IA_Zoom"))
  (bind _springarm1 (`self.SpringArm1`))
  (bind _springarm (`self.SpringArm`))
  ; Zoom
  (:`Triggered`
    (if (`ActorComponent.IsActive` (`self.Camera`))
      (set `SpringArmComponent.TargetArmLength` (`KismetMathLibrary.FClamp` (- (`SpringArmComponent.TargetArmLength` _springarm) (* ActionValue 10.0)) 250.0 700.0) _springarm)
      (else
        (set `SpringArmComponent.TargetArmLength` (`KismetMathLibrary.FClamp` (- (`SpringArmComponent.TargetArmLength` _springarm1) (* ActionValue 20.0)) 500.0 1500.0) _springarm1)))))

(event `self.ReceiveBeginPlay`
  (message `EnhancedInputSubsystemInterface.AddMappingContext` (pcsubsystem `EnhancedInputLocalPlayerSubsystem` (`GameplayStatics.GetPlayerController` 0)) "/Game/Input/IMC_Player.IMC_Player" 0 (struct))
  (bind _returnvalue (`|CreateWidget` "/Game/Player/WBP_Minimap.WBP_Minimap_C"))
  (`UserWidget.AddToViewport` _returnvalue 0))

(event `EnhancedInput|/Game/Input/IA_Crouch`
  (params (ActionValue :type Boolean) (ElapsedSeconds :type "Float (double-precision)") (TriggeredSeconds :type "Float (double-precision)") (InputAction :type "InputAction Object Reference" :default "/Game/Input/IA_Crouch.IA_Crouch"))
  ; Movement
  (:`Triggered`
    (`self.Crouch`))
  (:`Completed`
    (`self.UnCrouch`)))

(event `EnhancedInput|/Game/Input/IA_Move`
  (params (ActionValue :type "Vector2D Structure") (ElapsedSeconds :type "Float (double-precision)") (TriggeredSeconds :type "Float (double-precision)") (InputAction :type "InputAction Object Reference" :default "/Game/Input/IA_Move.IA_Move"))
  (bind (_returnvalue_roll _returnvalue_pitch _returnvalue_yaw) (`KismetMathLibrary.BreakRotator` (`self.GetControlRotation`)))
  ; Movement
  (:`Triggered`
    (if (`ActorComponent.IsActive` (`self.Camera`))
      (`self.AddMovementInput` (`KismetMathLibrary.GetRightVector` (`KismetMathLibrary.MakeRotator` 0.0 0.0 _returnvalue_yaw)) ActionValue_X)
      (`self.AddMovementInput` (`KismetMathLibrary.GetForwardVector` (`KismetMathLibrary.MakeRotator` 0.0 0.0 _returnvalue_yaw)) ActionValue_Y))))

(event `EnhancedInput|/Game/Input/IA_Look`
  (params (ActionValue :type "Vector2D Structure") (ElapsedSeconds :type "Float (double-precision)") (TriggeredSeconds :type "Float (double-precision)") (InputAction :type "InputAction Object Reference" :default "/Game/Input/IA_Look.IA_Look"))
  ; Movement
  (:`Triggered`
    (if (`ActorComponent.IsActive` (`self.Camera`))
      (`self.AddControllerYawInput` ActionValue_X)
      (bind _result (`/Engine/EditorBlueprintResources/StandardMacros.NegateFloat` ActionValue_Y)
        (:`  `
          (`self.AddControllerPitchInput` _result))))))

(event `EnhancedInput|/Game/Input/IA_Jump`
  (params (ActionValue :type Boolean) (ElapsedSeconds :type "Float (double-precision)") (TriggeredSeconds :type "Float (double-precision)") (InputAction :type "InputAction Object Reference" :default "/Game/Input/IA_Jump.IA_Jump"))
  ; Movement
  (:`Triggered`
    (`self.Jump`)))

(event `EnhancedInput|/Game/Input/IA_SwitchCam`
  (params (ActionValue :type Boolean) (ElapsedSeconds :type "Float (double-precision)") (TriggeredSeconds :type "Float (double-precision)") (InputAction :type "InputAction Object Reference" :default "/Game/Input/IA_SwitchCam.IA_SwitchCam"))
  (bind _camera1 (`self.Camera1`))
  (bind _camera (`self.Camera`))
  (:`Started`
    (if (`ActorComponent.IsActive` (`self.Camera1`))
      (set `PlayerController.bShowMouseCursor` false (`GameplayStatics.GetPlayerController` 0))
      (`ActorComponent.SetActive` _camera1 false false)
      (`ActorComponent.SetActive` _camera true false)
      (else
        (set `PlayerController.bShowMouseCursor` true (`GameplayStatics.GetPlayerController` 0))
        (`ActorComponent.SetActive` _camera false false)
        (`ActorComponent.SetActive` _camera1 true false)))))

(event `EnhancedInput|/Game/Input/IA_MoveTo`
  (params (ActionValue :type Boolean) (ElapsedSeconds :type "Float (double-precision)") (TriggeredSeconds :type "Float (double-precision)") (InputAction :type "InputAction Object Reference" :default "/Game/Input/IA_MoveTo.IA_MoveTo"))
  ; Topdown
  (:`Started`
    (if (`ActorComponent.IsActive` (`self.Camera1`))
      (set `self.TargetLocation` (`.Location` (`GameplayStatics.BreakHitResult` (`PlayerController.GetHitResultUnderCursorByChannel` (`GameplayStatics.GetPlayerController` 0) "TraceTypeQuery1" true))))
      (set `self.Walking` true))))

(event `self.ReceiveTick`
  (params (DeltaSeconds :type "Float (single-precision)"))
  (bind _returnvalue (`self.K2_GetActorLocation`))
  (bind _targetlocation (`self.TargetLocation`))
  (bind _returnvalue_2 (- _targetlocation _returnvalue))
  ; Topdown
  (if (`self.Walking`)
    (if (> (`KismetMathLibrary.VSize` _returnvalue_2) 100.0)
      (`self.AddMovementInput` (* (`KismetMathLibrary.Normal` _returnvalue_2) (* (`MovementComponent.GetMaxSpeed` (`self.CharacterMovement`)) DeltaSeconds)))
      (`self.K2_SetActorRotation` (`KismetMathLibrary.MakeRotator` 0.0 0.0 (.yaw (`KismetMathLibrary.FindLookAtRotation` _returnvalue _targetlocation))))
      (else
        (set `self.Walking` false)))))

(event `EnhancedInput|/Game/Input/IA_Sprint`
  (params (ActionValue :type Boolean) (ElapsedSeconds :type "Float (double-precision)") (TriggeredSeconds :type "Float (double-precision)") (InputAction :type "InputAction Object Reference" :default "/Game/Input/IA_Sprint.IA_Sprint"))
  (bind _charactermovement (`self.CharacterMovement`))
  (:`Started`
    (set `self.Running` true)
    (set `CharacterMovementComponent.MaxWalkSpeed` 900.0 _charactermovement))
  (:`Canceled`
    (set `self.Running` true :!label _label)
    (set `CharacterMovementComponent.MaxWalkSpeed` 600.0 _charactermovement))
  (:`Completed`
    (goto _label)))

(event `EnhancedInput|/Game/Input/IA_Interact`
  (params (ActionValue :type Boolean) (ElapsedSeconds :type "Float (double-precision)") (TriggeredSeconds :type "Float (double-precision)") (InputAction :type "InputAction Object Reference" :default "/Game/Input/IA_Interact.IA_Interact"))
  (bind _returnvalue (`GameplayStatics.GetPlayerController` 0))
  (bind (_sizex _sizey) (`PlayerController.GetViewportSize` _returnvalue))
  (bind (_worldposition _worlddirection) (`GameplayStatics.DeprojectScreenToWorld` _returnvalue (`KismetMathLibrary.MakeVector2D` (`KismetMathLibrary.Conv_IntToDouble` (/ _sizex 2)) (`KismetMathLibrary.Conv_IntToDouble` (/ _sizey 2)))))
  (:`Started`
    (bind _outhit (`KismetSystemLibrary.LineTraceSingle` _worldposition (+ _worldposition (* _worlddirection 500)) "TraceTypeQuery1"))
    (bind _asbp_interactable (cast `/Game/Player/BP_Interactable` (`.HitActor` (`GameplayStatics.BreakHitResult` _outhit))))
    (set `/Game/Player/BP_Interactable.Held` true _asbp_interactable)
    (set `self.Holding` true))
  (:`Completed`
    (if (`self.Holding`)
      (set `self.Holding` false)
      (set `/Game/Player/BP_Interactable.Held` false _asbp_interactable))))

(event `EnhancedInput|/Game/Input/IA_Aim`
  (params (ActionValue :type Boolean) (ElapsedSeconds :type "Float (double-precision)") (TriggeredSeconds :type "Float (double-precision)") (InputAction :type "InputAction Object Reference" :default "/Game/Input/IA_Aim.IA_Aim"))
  (bind _camera (`self.Camera`))
  (bind _charactermovement (`self.CharacterMovement`))
  (:`Started`
    (set `self.Aiming` true)
    (`CameraComponent.SetFieldOfView` _camera 60.0)
    (set `CharacterMovementComponent.MaxWalkSpeed` 400.0 _charactermovement))
  (:`Canceled`
    (set `self.Aiming` false :!label _label_2)
    (`CameraComponent.SetFieldOfView` _camera 90.0)
    (set `CharacterMovementComponent.MaxWalkSpeed` 600.0 _charactermovement))
  (:`Completed`
    (goto _label_2)))

(event `EnhancedInput|/Game/Input/IA_Shoot`
  (params (ActionValue :type Boolean) (ElapsedSeconds :type "Float (double-precision)") (TriggeredSeconds :type "Float (double-precision)") (InputAction :type "InputAction Object Reference" :default "/Game/Input/IA_Shoot.IA_Shoot"))
  (bind _returnvalue (`KismetMathLibrary.MakeTransform` (`SceneComponent.K2_GetComponentLocation` (`self.Wand`)) (`PlayerCameraManager.GetCameraRotation` (`GameplayStatics.GetPlayerCameraManager` 0))))
  (:`Triggered`
    (if (`self.Aiming`)
      (if (not (`self.ShootCooldown`))
        (set `self.ShootCooldown` true)
        (if (`self.ProjectileType`)
          (`|SpawnActorFromClass` "/Game/Player/BP_Projectile2.BP_Projectile2_C" _returnvalue "Undefined" "MultiplyWithRoot" null null)
          (`KismetSystemLibrary.Delay` 1.0)
          (set `self.ShootCooldown` false)
          (else
            (`|SpawnActorFromClass` "/Game/Player/BP_Projectile.BP_Projectile_C" _returnvalue "Undefined" "MultiplyWithRoot" null null)
            (`KismetSystemLibrary.Delay` 0.5)
            (set `self.ShootCooldown` false)))))))

(event `EnhancedInput|/Game/Input/IA_SwitchProj`
  (params (ActionValue :type Boolean) (ElapsedSeconds :type "Float (double-precision)") (TriggeredSeconds :type "Float (double-precision)") (InputAction :type "InputAction Object Reference" :default "/Game/Input/IA_SwitchProj.IA_SwitchProj"))
  (:`Started`
    (if (`self.ProjectileType`)
      (set `self.ProjectileType` false)
      (else
        (set `self.ProjectileType` true)))))

(fn `UserConstructionScript`)