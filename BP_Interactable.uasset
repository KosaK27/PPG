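; BP_Interactable is an actor that can be carried in front of the player's view while its Held flag is true.
; Each tick while held, it deprojects the viewport center of player 0 and moves itself a fixed distance along that ray.
; The move does not sweep for collision, and nothing in this graph sets Held.
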(event `self.ReceiveTick`
  (params (DeltaSeconds :type "Float (single-precision)"))
  (bind _returnvalue (`GameplayStatics.GetPlayerController` 0))
  (bind (_sizex _sizey) (`PlayerController.GetViewportSize` _returnvalue))
  (bind (_worldposition _worlddirection) (`GameplayStatics.DeprojectScreenToWorld` _returnvalue (`KismetMathLibrary.MakeVector2D` (`KismetMathLibrary.Conv_IntToDouble` (/ _sizex 2)) (`KismetMathLibrary.Conv_IntToDouble` (/ _sizey 2)))))
  (if (`self.Held`)
    (`self.K2_SetActorLocation` (+ _worldposition (* _worlddirection 500)))))

(fn `UserConstructionScript`)