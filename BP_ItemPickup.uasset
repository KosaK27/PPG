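; BP_ItemPickup is a pickup actor that adds an item to the player's inventory when hit.
; A hit on Sphere1 by BP_TestPlayer builds an STItem from the pickup's ID, Name, Icon and Quantity variables and passes it to BPInventoryComponent.
; It then plays a sound at world origin, destroys itself and prints a debug message.
; On BeginPlay, it applies its Material variable to Sphere after a short delay.
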(event `self.Sphere1.OnComponentHit`
  (params (HitComponent :type "PrimitiveComponent Object Reference") (OtherActor :type "Actor Object Reference") (OtherComp :type "PrimitiveComponent Object Reference") (NormalImpulse :type "Vector Structure") (Hit :type "HitResult Structure (by ref)"))
  (bind _asbp_test_player (cast `/Game/Player/BP_TestPlayer` OtherActor))
  (`/Game/Player/BP_InventoryComponent.AddItem` (`/Game/Player/BP_TestPlayer.BP_InventoryComponent` _asbp_test_player) (make `/Game/Player/ST_Item` (`self.ID`) (`self.Name`) (`self.Icon`) (`self.Quantity`)))
  (`GameplayStatics.PlaySoundAtLocation` "/Engine/VREditor/Sounds/UI/Floating_UI_Close-001.Floating_UI_Close-001" (0.0 0.0 0.0) (struct) 1.0 1.0 0.0 null null null null)
  (`self.K2_DestroyActor`)
  (`KismetSystemLibrary.PrintString` "Item1 Pickup"))

(event `self.ReceiveBeginPlay`
  (`KismetSystemLibrary.Delay` 0.1)
  (`PrimitiveComponent.SetMaterial` (`self.Sphere`) 0 (`self.Material`)))

(fn `UserConstructionScript`)