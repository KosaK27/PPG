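; BP_PickupSpawner scatters randomized item pickups across the area of its static mesh when play begins.
; For each class in the Pickup array, it spawns two to five actors at random XY points within the mesh bounds, at a fixed world height.
; Each BP_ItemPickup gets a random ID that sets its name and indexes the icon and material arrays, plus a random quantity.
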(event `self.ReceiveBeginPlay`
  (bind (_origin _boxextent) (`KismetSystemLibrary.GetComponentBounds` (`self.StaticMesh`)))
  (bind _x (.x _boxextent))
  (bind _y (.y _boxextent))
  (bind _x_2 (.x _origin))
  (bind _y_2 (.y _origin))
  (for _array_element (`self.Pickup`)
    (for _ (range (+ (`KismetMathLibrary.RandomIntegerInRange` 2 5) 1))
      (bind _returnvalue (`|SpawnActorFromClass` _array_element (`KismetMathLibrary.MakeTransform` (`KismetMathLibrary.MakeVector` (`KismetMathLibrary.RandomFloatInRange` (- _x_2 _x) (+ _x_2 _x)) (`KismetMathLibrary.RandomFloatInRange` (- _y_2 _y) (+ _y_2 _y)) 100.0)) "Undefined" "MultiplyWithRoot" null null))
      (bind _asbp_item_pickup (cast `/Game/Player/BP_ItemPickup` _returnvalue))
      (bind _output_get (set `/Game/Player/BP_ItemPickup.ID` (`KismetMathLibrary.RandomIntegerInRange` 0 1) _asbp_item_pickup))
      (set `/Game/Player/BP_ItemPickup.Name` (`KismetStringLibrary.Concat_StrStr` "Item" (`KismetStringLibrary.Conv_IntToString` _output_get)) _asbp_item_pickup)
      (set `/Game/Player/BP_ItemPickup.Icon` (`|GetArrayItem` (`self.Icons`) _output_get) _asbp_item_pickup)
      (set `/Game/Player/BP_ItemPickup.Quantity` (`KismetMathLibrary.RandomIntegerInRange` 1 3) _asbp_item_pickup)
      (set `/Game/Player/BP_ItemPickup.Material` (`|GetArrayItem` (`self.Materials`) _output_get) _asbp_item_pickup))))

(fn `UserConstructionScript`)